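; Arcane Shards gameplay ability that bursts shards at shuffled ground points around a player-confirmed target location.
; A circle indicator target actor supplies the location, then a cast montage plays until its attack gameplay event fires.
; The server then generates radial points with random yaw, and a looping timer triggers a gameplay cue at each before ending the ability.
; Debug spheres mark the points; no damage is applied here.
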(event `self.K2_ActivateAbility`
  (bind (_asynctaskproxy _data) (`AbilityTask_WaitTargetData.WaitTargetData` "None" "UserConfirmed" "/Game/Blueprints/AbilitySystem/TargetActor/BP_CircleIndicator.BP_CircleIndicator_C" (struct) (struct) null)
    (:`ValidData`
      (`KismetSystemLibrary.PrintString` "Confirm ability")
      (`AbilityTask_PlayMontageAndWait.CreatePlayMontageAndWaitProxy` "None" "/Game/Assets/Characters/Aura/Animations/Abilities/AM_Cast_ArcaneShards.AM_Cast_ArcaneShards"
        (:`then`
          (`AbilityTask_WaitGameplayEvent.WaitGameplayEvent` (struct :`TagName` "Montage.Attack") null true false
            (:`EventReceived`
              (`self.K2_HasAuthority`
                (:`True`
                  (`KismetSystemLibrary.Delay` 0.01)
                  (bind _returnvalue (`RPGAbilitySystemLibrary.GetGroundRadialPoints` null (`AbilitySystemBlueprintLibrary.GetTargetDataEndPoint` _data) (`self.NumPoints`) 200.0 (`KismetMathLibrary.RandomFloatInRange` 0.0 360.0)))
                  (bind _output_get (set `self.SpawnPoints` _returnvalue))
                  (`KismetArrayLibrary.Array_Shuffle` _output_get)
                  (bind _returnvalue_2 (`KismetSystemLibrary.K2_SetTimerDelegate` (delegate `SpawnShard`) (`self.ShardSpawnDeltaTime`) true))
                  (set `self.ShardSpawnTimer` _returnvalue_2)
                  (`self.SpawnShard`))))))))
    (:`Cancelled`
      (`KismetSystemLibrary.PrintString` "cancel ability")
      (`self.K2_EndAbility`))))

(event `SpawnShard`
  (bind _output (`|GetArrayItem` (`self.SpawnPoints`) (`self.Count`)))
  (if (< (`self.Count`) (`self.NumPoints`))
    (`self.K2_ExecuteGameplayCueWithParams` (struct :`TagName` "GameplayCue.ShardsBurst") (`AbilitySystemBlueprintLibrary.MakeGameplayCueParameters` 0.0 0.0 (struct) (struct) (struct) (struct) (struct) _output))
    (`KismetSystemLibrary.DrawDebugSphere` _output 50.0 12 (struct :`R` 1.0 :`A` 1.0) 5.0)
    (`/Engine/EditorBlueprintResources/StandardMacros.IncrementInt` (`self.Count`))
    (else
      (`KismetSystemLibrary.K2_ClearAndInvalidateTimerHandle` (`self.ShardSpawnTimer`))
      (`self.K2_EndAbility`))))