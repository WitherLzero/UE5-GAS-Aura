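; GA_FireBolt is the Aura gameplay ability that casts a Fire Bolt projectile toward the location under the mouse.
; On activation, an ability task supplies the cursor's target data, and the hit location is passed to the ActionComponent to update the facing target.
; It then plays the cast montage and waits for the montage's gameplay event to spawn the projectile at that target, ending after a short delay.
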(event `self.K2_ActivateAbility`
  (bind (_asynctaskproxy _datahandle) (`TargetDataUnderMouse.CreateTargetDataUnderMouse`)
    (:`ValidData`
      (set `self.ProjectileTargetLoc` (`.Location` (`GameplayStatics.BreakHitResult` (`AbilitySystemBlueprintLibrary.GetHitResultFromTargetData` _datahandle))))
      (bind _actioncomponent (`self.ActionComponent`)
        (:`then`
          (`ActionComponent.UpdateFacingTarget` _actioncomponent (`self.ProjectileTargetLoc`))
          (`AbilityTask_PlayMontageAndWait.CreatePlayMontageAndWaitProxy` "None" "/Game/Assets/Characters/Aura/Animations/Abilities/AM_Cast_FireBolt.AM_Cast_FireBolt"
            (:`then`
              (`AbilityTask_WaitGameplayEvent.WaitGameplayEvent` (struct :`TagName` "Event.Montage.FireBolt") null
                (:`EventReceived`
                  (`self.SpawnProjectile` (`self.ProjectileTargetLoc`))
                  (`KismetSystemLibrary.Delay` 0.5)
                  (`self.K2_EndAbility`))))))
        (:`else`)))))