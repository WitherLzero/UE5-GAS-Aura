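; Electrocute gameplay ability for Aura: a held lightning cast toward the mouse target, with no damage logic in this graph.
; On activation it stores the cursor hit, hides the cursor, turns the caster to face it, fires a ShockBurst cue and plays the cast montage.
; The montage's weapon event adds a looping shock cue with the weapon and hit location.
; Input release restores the cursor, removes the loop and ends the ability.
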(event `self.K2_ActivateAbility`
  (bind _returnvalue (`self.GetAvatarActorFromActorInfo`))
  (set `self.PlayerController` (`.PlayerController` (break `GameplayAbilityActorInfo` (`self.GetActorInfo`))))
  (bind (_asynctaskproxy _datahandle) (`TargetDataUnderMouse.CreateTargetDataUnderMouse`)
    (:`ValidData`
      (`self.StoreMouseDataInfo` (`AbilitySystemBlueprintLibrary.GetHitResultFromTargetData` _datahandle))
      (`|ExecutionSequence`
        (:`then_0`
          (set `PlayerController.bShowMouseCursor` false (`self.PlayerController`))
          (bind _actioncomponent (`self.ActionComponent`)
            (:`then`
              (`ActionComponent.UpdateFacingTarget` _actioncomponent (`self.MouseHitLocation`))
              (`self.K2_ExecuteGameplayCue` (struct :`TagName` "GameplayCue.ShockBurst"))
              (`AbilityTask_PlayMontageAndWait.CreatePlayMontageAndWaitProxy` "None" "/Game/Assets/Characters/Aura/Animations/Abilities/AM_Cast_Shock.AM_Cast_Shock" 1.0 "None" false
                (:`then`
                  (`AbilityTask_WaitGameplayEvent.WaitGameplayEvent` (struct :`TagName` "Montage.Attack.Weapon") null
                    (:`EventReceived`
                      (`GameplayCueFunctionLibrary.AddGameplayCueOnActor` _returnvalue (struct :`TagName` "GameplayCue.ShockLoop") (`AbilitySystemBlueprintLibrary.MakeGameplayCueParameters` 0.0 0.0 (struct) (struct) (struct) (struct) (struct) (`self.MouseHitLocation`) (0.0 0.0 0.0) null null null null 1 1 (`RPGAbilitySystemLibrary.GetWeapon` _returnvalue))))))))
            (:`else`)))
        (:`then_1`
          (`AbilityTask_WaitInputRelease.WaitInputRelease` false
            (:`OnRelease`
              (set `PlayerController.bShowMouseCursor` true (`self.PlayerController`))
              (`self.K2_RemoveGameplayCue` (struct :`TagName` "GameplayCue.ShockLoop"))
              (`self.K2_EndAbility`))))))))