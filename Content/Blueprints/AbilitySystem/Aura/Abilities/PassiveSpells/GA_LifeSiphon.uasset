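; GA_LifeSiphon is a passive Gameplay Ability that keeps the Life Siphon gameplay effect active on its owner.
; On activation it applies GE_Activate_LifeSiphon at the ability's level and stores the handle.
; It binds to the RPG Ability System Component's level-changed delegate to update the active effect's level in place.
; When the ability ends, it removes the effect by that handle.
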(event `self.K2_ActivateAbility`
  (bind _returnvalue (`self.BP_ApplyGameplayEffectToOwner` "/Game/Blueprints/AbilitySystem/Aura/Abilities/PassiveSpells/GE/GE_Activate_LifeSiphon.GE_Activate_LifeSiphon_C" (`self.GetAbilityLevel`)))
  (set `self.LifeSiphon` _returnvalue)
  (bind _asrpgability_system_component (cast `RPGAbilitySystemComponent` (`self.GetAbilitySystemComponentFromActorInfo`)))
  (add `RPGAbilitySystemComponent.OnAbilityLevelChanged` _asrpgability_system_component (delegate `OnAbilityLevelChanged_Event`)))

(event `OnAbilityLevelChanged_Event`
  (`AbilitySystemComponent.SetActiveGameplayEffectLevel` (`self.GetAbilitySystemComponentFromActorInfo`) (`self.LifeSiphon`) (`self.GetAbilityLevel`)))

(event `self.K2_OnEndAbility`
  (params (bWasCancelled :type Boolean))
  (`self.BP_RemoveGameplayEffectFromOwnerWithHandle` (`self.LifeSiphon`)))