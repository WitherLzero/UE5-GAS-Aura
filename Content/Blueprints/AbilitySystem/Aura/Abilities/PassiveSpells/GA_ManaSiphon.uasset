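; GA_ManaSiphon is a passive gameplay ability for the Aura character that grants the Mana Siphon effect while active.
; On activation it applies GE_Activate_ManaSiphon at the ability's level and stores the effect handle.
; It binds to the RPG ability system component's level-change delegate to update that active effect's level in place.
; When the ability ends, it removes all stacks of the effect by handle.
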(event `self.K2_ActivateAbility`
  (bind _returnvalue (`self.BP_ApplyGameplayEffectToOwner` "/Game/Blueprints/AbilitySystem/Aura/Abilities/PassiveSpells/GE/GE_Activate_ManaSiphon.GE_Activate_ManaSiphon_C" (`self.GetAbilityLevel`)))
  (set `self.ManaSiphon` _returnvalue)
  (bind _asrpgability_system_component (cast `RPGAbilitySystemComponent` (`self.GetAbilitySystemComponentFromActorInfo`)))
  (add `RPGAbilitySystemComponent.OnAbilityLevelChanged` _asrpgability_system_component (delegate `OnAbilityLevelChanged_Event`)))

(event `OnAbilityLevelChanged_Event`
  (`AbilitySystemComponent.SetActiveGameplayEffectLevel` (`self.GetAbilitySystemComponentFromActorInfo`) (`self.ManaSiphon`) (`self.GetAbilityLevel`)))

(event `self.K2_OnEndAbility`
  (params (bWasCancelled :type Boolean))
  (`self.BP_RemoveGameplayEffectFromOwnerWithHandle` (`self.ManaSiphon`)))