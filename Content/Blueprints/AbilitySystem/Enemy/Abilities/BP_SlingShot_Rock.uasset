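; BP_SlingShot_Rock is the rock actor for an enemy slingshot ability, giving its mesh a random tumbling spin.
; BeginPlay picks random positive or negative yaw, pitch and roll rates for each instance.
; Tick applies those rates, scaled by delta time, as local rotation on RockMesh.
; The graphs handle only this visual spin, with no movement, overlap or damage logic.
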(event `self.ReceiveBeginPlay`
  (bind _returnvalue (`KismetMathLibrary.RandomFloatInRange` -500.0 500.0))
  (set `self.YawRotRate` _returnvalue)
  (set `self.PitchRotRate` _returnvalue)
  (set `self.RollRotRate` _returnvalue))

(event `self.ReceiveTick`
  (params (DeltaSeconds :type "Float (single-precision)"))
  (`SceneComponent.K2_AddLocalRotation` (`self.RockMesh`) (* (`KismetMathLibrary.MakeRotator` (`self.RollRotRate`) (`self.PitchRotRate`) (`self.YawRotRate`)) DeltaSeconds) false false))

(fn `UserConstructionScript`)