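; Enemy gameplay ability that performs a melee attack on live players.
; It turns the avatar toward its combat target and plays a random tagged montage from the CombatComponent.
; The montage's tag drives both the awaited gameplay event and the socket lookup for a small-radius search, damaging each player found.
; The ability ends when the montage completes, is interrupted or is cancelled.
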(event `self.K2_ActivateAbility`
  (bind _returnvalue (`self.GetAvatarActorFromActorInfo`))
  (bind _combatcomponent (`self.CombatComponent`)
    (:`then`
      (bind _actioncomponent (`self.ActionComponent`)
        (:`then`
          (`ActionComponent.UpdateFacingTarget` _actioncomponent (`Actor.K2_GetActorLocation` (`CombatComponent.GetCombatTarget` _combatcomponent)))
          (bind _returnvalue_2 (`CombatComponent.GetAttackMontages` (`self.CombatComponent`)))
          (bind _returnvalue_3 (`RPGAbilitySystemLibrary.PickRandomTaggedMontage` _returnvalue_2))
          (bind (_montage _montagetag) (break `TaggedMontage` _returnvalue_3))
          (`AbilityTask_PlayMontageAndWait.CreatePlayMontageAndWaitProxy` "None" _montage
            (:`then`
              (`AbilityTask_WaitGameplayEvent.WaitGameplayEvent` _montagetag null
                (:`EventReceived`
                  (bind _outoverlappingactors (`RPGAbilitySystemLibrary.GetLivePlayersWithinRadius` _returnvalue (`|MakeArray` _returnvalue) 30.0 (`CombatComponent.GetCombatSocketLocation` (`self.CombatComponent`) _montagetag)))
                  (for _array_element _outoverlappingactors
                    (`self.CauseDamage` _array_element)))))
            (:`OnCompleted`
              (`self.K2_EndAbility` :!label _label))
            (:`OnInterrupted`
              (goto _label))
            (:`OnCancelled`
              (goto _label))))
        (:`else`)))
    (:`else`)))