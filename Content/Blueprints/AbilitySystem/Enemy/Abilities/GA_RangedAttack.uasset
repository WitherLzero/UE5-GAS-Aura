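; GA_RangedAttack is an enemy gameplay ability that fires a projectile at the avatar's combat target.
; On activation it captures the target's location, updates facing toward it through the ActionComponent, and plays a random tagged attack montage.
; The montage's gameplay event spawns the projectile from the matching combat socket toward the captured location, with class-default damage effect params.
; The ability ends when the montage completes, is interrupted or is cancelled.
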(event `self.K2_ActivateAbility`
  (bind _returnvalue (`self.GetAvatarActorFromActorInfo`))
  (set `self.TargetLoc` (`Actor.K2_GetActorLocation` (`RPGAbilitySystemLibrary.GetCombatTarget` _returnvalue)))
  (bind _actioncomponent (`self.ActionComponent`)
    (:`then`
      (`ActionComponent.UpdateFacingTarget` _actioncomponent (`self.TargetLoc`))
      (bind _returnvalue_2 (`RPGAbilitySystemLibrary.PickRandomTaggedMontage` (`RPGAbilitySystemLibrary.GetAttackMontages` _returnvalue)))
      (bind (_montage _montagetag) (break `TaggedMontage` _returnvalue_2))
      (`AbilityTask_PlayMontageAndWait.CreatePlayMontageAndWaitProxy` "None" _montage
        (:`then`
          (bind (_asynctaskproxy _payload) (`AbilityTask_WaitGameplayEvent.WaitGameplayEvent` _montagetag null false false)
            (:`EventReceived`
              (bind (_eventtag _instigator) (break `GameplayEventData` _payload))
              (`RPGAbilitySystemLibrary.SpawnProjectileTowardsTarget` null (`self.ProjectileClass`) (`RPGAbilitySystemLibrary.GetCombatSocketLocation` _instigator _eventtag) (`self.TargetLoc`) false 0.0 (`self.GetAvatarActorFromActorInfo`) (`self.MakeDamageEffectParamsFromClassDefaults` null)))))
        (:`OnCompleted`
          (`self.K2_EndAbility` :!label _label))
        (:`OnInterrupted`
          (goto _label))
        (:`OnCancelled`
          (goto _label))))
    (:`else`)))