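; Gameplay ability for an enemy, apparently a Shaman, that summons random minions at shuffled locations.
; Activation shows ground effects at each location and plays the summon montage, whose Montage.Attack event starts staggered spawning of AI-controlled minions via a delayed loop.
; Each minion applies a GE_MinionTracker effect to the owner, mapped by actor so its death removes that effect.
; The ability ends when the montage completes or is interrupted or cancelled.
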(event `self.K2_ActivateAbility`
  (set `self.Index` 0)
  (bind _returnvalue (`self.GetSummonLocations`))
  (bind _output_get (set `self.SummonLocations` _returnvalue))
  (`KismetArrayLibrary.Array_Shuffle` _output_get)
  (for _array_element (`self.SummonLocations`)
    (`NiagaraFunctionLibrary.SpawnSystemAtLocation` "/Game/Assets/Effects/Combat/NS_GroundSummon.NS_GroundSummon" _array_element))
  (`AbilityTask_PlayMontageAndWait.CreatePlayMontageAndWaitProxy` "None" "/Game/Assets/Enemies/Shaman/Animations/AM_Shaman_Summon.AM_Shaman_Summon"
    (:`then`
      (`AbilityTask_WaitGameplayEvent.WaitGameplayEvent` (struct :`TagName` "Montage.Attack") null
        (:`EventReceived`
          (if (< (`self.Index`) (`KismetArrayLibrary.Array_Length` (`self.SummonLocations`))) :!label _label
            (bind _returnvalue_2 (`|SpawnActorFromClass` (`self.PickRandomMinionClass`) (`KismetMathLibrary.MakeTransform` (+ (`|GetArrayItem` (`self.SummonLocations`) (`self.Index`)) (0.0 0.0 50.0)) (`Actor.K2_GetActorRotation` (`self.GetAvatarActorFromActorInfo`))) "AdjustIfPossibleButAlwaysSpawn" "MultiplyWithRoot" null null))
            (`Pawn.SpawnDefaultController` _returnvalue_2)
            (add `VitalityComponent.OnDeath` (`Actor.GetComponentByClass` _returnvalue_2 "/Script/Aura.VitalityComponent") (delegate `Decrement Minion Count`))
            (bind _returnvalue_3 (`self.BP_ApplyGameplayEffectToOwner` "/Game/Blueprints/AbilitySystem/Enemy/Effects/GE_MinionTracker.GE_MinionTracker_C"))
            (`BlueprintMapLibrary.Map_Add` (`self.ActorToEffectHandle`) _returnvalue_2 _returnvalue_3)
            (`/Engine/EditorBlueprintResources/StandardMacros.IncrementInt` (`self.Index`)
              (:`  `
                (`KismetSystemLibrary.Delay` 0.2)
                (goto _label)))))))
    (:`OnCompleted`
      (`self.K2_EndAbility` :!label _label_2))
    (:`OnInterrupted`
      (goto _label_2))
    (:`OnCancelled`
      (goto _label_2))))

(event `Decrement Minion Count`
  (params (DeadActor :type "Actor Object Reference") (Instigator :type "Actor Object Reference"))
  (`self.BP_RemoveGameplayEffectFromOwnerWithHandle` (`BlueprintMapLibrary.Map_Find` (`self.ActorToEffectHandle`) DeadActor))
  (`BlueprintMapLibrary.Map_Remove` (`self.ActorToEffectHandle`) DeadActor))